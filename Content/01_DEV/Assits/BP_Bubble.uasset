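; BP_Bubble is a bubble actor that drifts its BubbleDarkBlue component around its starting position.
; BeginPlay caches the world location, starts a timeline and picks a random per-axis offset between Min and Max.
; The timeline's Loop track drives a normal-vector slerp between the cached location and the offset point.
; Each finish rolls a new offset and replays the timeline, so the motion repeats indefinitely around the same origin.
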(event `self.ReceiveBeginPlay`
  (bind _returnvalue (`KismetMathLibrary.RandomFloatInRange` (`self.Min`) (`self.Max`)))
  (set `self.Location` (`SceneComponent.K2_GetComponentLocation` (`self.Bubble_DarkBlue`)))
  (`self.Lerp`)
  (set `self.Random` (`KismetMathLibrary.MakeVector` _returnvalue _returnvalue _returnvalue)))

(event `Lerp`
  (bind _location (`self.Location`))
  (bind _returnvalue (`KismetMathLibrary.RandomFloatInRange` (`self.Min`) (`self.Max`)))
  (bind (_direction _loop) (`Timeline|Timeline` :!via `PlayFromStart`)
    (:`Update`
      (`SceneComponent.K2_SetWorldLocation` (`self.Bubble_DarkBlue`) (`KismetMathLibrary.Vector_SlerpNormals` _location (+ _location (`self.Random`)) _loop) false false))
    (:`Finished`
      (set `self.Random` (`KismetMathLibrary.MakeVector` _returnvalue _returnvalue _returnvalue))
      (`self.Lerp`))))

(fn `UserConstructionScript`)