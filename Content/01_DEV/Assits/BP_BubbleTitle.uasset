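; BP_BubbleTitle is a bubble, likely title decoration by its name, that animates its BubbleDarkBlue component along the world Z axis.
; BeginPlay stores the starting height and picks one random Z offset between Min and Max, so instances can travel different distances.
; A Timeline's Loop track interpolates between the start and offset heights, and its Finished output calls the Lerp event again to repeat indefinitely.
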(event `self.ReceiveBeginPlay`
  (bind (_returnvalue_x _returnvalue_y _returnvalue_z) (`KismetMathLibrary.BreakVector` (`SceneComponent.K2_GetComponentLocation` (`self.Bubble_DarkBlue`))))
  (set `self.Location` _returnvalue_z)
  (`self.Lerp`)
  (set `self.RandomZ` (`KismetMathLibrary.RandomFloatInRange` (`self.Min`) (`self.Max`))))

(event `Lerp`
  (bind (_returnvalue_x _returnvalue_y _returnvalue_z) (`KismetMathLibrary.BreakVector` (`SceneComponent.K2_GetComponentLocation` (`self.Bubble_DarkBlue`))))
  (bind (_direction _loop) (`Timeline|Timeline` :!via `PlayFromStart`)
    (:`Update`
      (`SceneComponent.K2_SetWorldLocation` (`self.Bubble_DarkBlue`) (`KismetMathLibrary.MakeVector` _returnvalue_x _returnvalue_y (`KismetMathLibrary.Lerp` (`self.Location`) (+ (`self.Location`) (`self.RandomZ`)) _loop)) false false))
    (:`Finished`
      (`self.Lerp`))))

(fn `UserConstructionScript`)