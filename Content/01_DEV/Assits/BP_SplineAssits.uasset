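; BP_SplineAssits is an actor that moves its Cube along its Spline in a continuous loop.
; Each Tick it places the cube at SplineDistance with the spline's world location and rotation, then advances that distance by SplineSpeed scaled by delta seconds.
; SplineForward sets the direction, and on passing either end the distance wraps to the opposite end rather than reversing.
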(event `self.ReceiveTick`
  (params (DeltaSeconds :type "Float (single-precision)"))
  (`self.Update Position`)
  (if (`self.SplineForward`)
    (if (< (`self.SplineDistance`) (`SplineComponent.GetSplineLength` (`self.Spline`)))
      (set `self.SplineDistance` (+ (`self.SplineDistance`) (* (`GameplayStatics.GetWorldDeltaSeconds`) (`self.SplineSpeed`))))
      (else
        (set `self.SplineDistance` 0.0)))
    (elif (> (`self.SplineDistance`) 0.0)
      (set `self.SplineDistance` (- (`self.SplineDistance`) (* (`GameplayStatics.GetWorldDeltaSeconds`) (`self.SplineSpeed`))))
      (else
        (set `self.SplineDistance` (`SplineComponent.GetSplineLength` (`self.Spline`)))))))

(event `Update Position`
  (bind _spline (`self.Spline`))
  (bind _cube (`self.Cube`))
  (bind _splinedistance (`self.SplineDistance`))
  (bind (_returnvalue_roll _returnvalue_pitch _returnvalue_yaw) (`KismetMathLibrary.BreakRotator` (`SplineComponent.GetRotationAtDistanceAlongSpline` _spline _splinedistance "World")))
  (`SceneComponent.K2_SetWorldLocation` _cube (`SplineComponent.GetLocationAtDistanceAlongSpline` _spline _splinedistance "World") false false)
  (`SceneComponent.K2_SetWorldRotation` _cube (`KismetMathLibrary.MakeRotator` _returnvalue_roll _returnvalue_pitch _returnvalue_yaw) false false))

(fn `UserConstructionScript`)