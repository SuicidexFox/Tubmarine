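; BP_Billboard is an actor that shows a randomly chosen, randomly sized material billboard with a looping vertical animation.
; On BeginPlay it adds one element to its MaterialBillboard from the material list, with width and height rolled separately between Min and Max.
; A timeline lerps the billboard's relative location from the origin toward a random Z offset, then restarts itself with a new offset on finish.
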(event `self.ReceiveBeginPlay`
  (bind _returnvalue (`KismetMathLibrary.Conv_IntToDouble` (`KismetMathLibrary.RandomIntegerInRange` (`self.Min`) (`self.Max`))))
  (`MaterialBillboardComponent.AddElement` (`self.MaterialBillboard`) (`|GetArrayItem` (`self.ListMaterial`) (`KismetMathLibrary.RandomInteger` (`KismetArrayLibrary.Array_Length` (`self.ListMaterial`)))) null false _returnvalue _returnvalue null)
  (`self.Animation`))

(event `Animation`
  (bind _output_get (set `self.B` (`KismetMathLibrary.MakeVector` 0.0 0.0 (`KismetMathLibrary.Conv_IntToDouble` (`KismetMathLibrary.RandomIntegerInRange` 20 50)))))
  (bind (_direction _alpha) (`Timeline|Timeline` :!via `PlayFromStart`)
    (:`Update`
      (`SceneComponent.K2_SetRelativeLocation` (`self.MaterialBillboard`) (`KismetMathLibrary.VLerp` (0.0 0.0 0.0) _output_get _alpha) false false))
    (:`Finished`
      (`self.Animation`))))

(fn `UserConstructionScript`)