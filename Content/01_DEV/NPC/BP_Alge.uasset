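; BP_Alge is an algae NPC that reacts to the BP_Nils character entering its Box trigger.
; While Nils is inside, it disables his jump, turns the Alge component toward him each tick and fades up its emissive via a timeline.
; Leaving sets jump velocity back, reverses the glow and reapplies the starting rotation.
; Touching the Alge itself launches Nils along his forward axis, scaled by Bounce.
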(event `self.ReceiveBeginPlay`
  (set `self.Rotation` (`SceneComponent.RelativeRotation` (`self.Alge`))))

(event `self.ReceiveTick`
  (params (DeltaSeconds :type "Float (single-precision)"))
  (if (`self.Rotator`)
    (`SceneComponent.K2_SetWorldRotation` (`self.Alge`) (`KismetMathLibrary.ComposeRotators` (`KismetMathLibrary.FindLookAtRotation` (`SceneComponent.K2_GetComponentLocation` (`self.Alge`)) (`self.K2_GetActorLocation` (stale `self.Box.OnComponentBeginOverlap` OtherActor))) (struct :`Yaw` 180.0)) false false)))

(event `self.Box.OnComponentBeginOverlap`
  (params (OverlappedComponent :type "PrimitiveComponent Object Reference") (OtherActor :type "Actor Object Reference") (OtherComp :type "PrimitiveComponent Object Reference") (OtherBodyIndex :type Integer) (bFromSweep :type Boolean) (SweepResult :type "HitResult Structure (by ref)"))
  (bind _asbp_nils (cast `/Game/01_DEV/Nils/BP_Nils` OtherActor))
  (set `CharacterMovementComponent.JumpZVelocity` 0.0 (`Character.CharacterMovement` _asbp_nils))
  (set `self.Rotator` true)
  (bind (_direction _growth) (`Timeline|Ani` :!label _label)
    (:`Update`
      (bind _output_get (set `self.AniTime` _growth))
      (`MeshComponent.SetScalarParameterValueOnMaterials` (`self.Alge`) "Emissive" _output_get))))

(event `self.Box.OnComponentEndOverlap`
  (params (OverlappedComponent :type "PrimitiveComponent Object Reference") (OtherActor :type "Actor Object Reference") (OtherComp :type "PrimitiveComponent Object Reference") (OtherBodyIndex :type Integer))
  (bind _asbp_nils (cast `/Game/01_DEV/Nils/BP_Nils` OtherActor))
  (set `CharacterMovementComponent.JumpZVelocity` 600.0 (`Character.CharacterMovement` _asbp_nils))
  (set `self.Rotator` false)
  (`|ExecutionSequence`
    (:`then_0`
      (goto _label :!via `Reverse`))
    (:`then_1`
      (`SceneComponent.K2_SetWorldRotation` (`self.Alge`) (`self.Rotation`) false false))))

(event `self.Alge.OnComponentBeginOverlap`
  (params (OverlappedComponent :type "PrimitiveComponent Object Reference") (OtherActor :type "Actor Object Reference") (OtherComp :type "PrimitiveComponent Object Reference") (OtherBodyIndex :type Integer) (bFromSweep :type Boolean) (SweepResult :type "HitResult Structure (by ref)"))
  ;[1 0.8137 0.1823] Bounce
  (bind _asbp_nils (cast `/Game/01_DEV/Nils/BP_Nils` OtherActor))
  (`Character.LaunchCharacter` _asbp_nils (* (`self.GetActorForwardVector` _asbp_nils) (`self.Bounce`)) true false))

(fn `UserConstructionScript`)