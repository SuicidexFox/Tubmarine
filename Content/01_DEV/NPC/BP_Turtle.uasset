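; Turtle NPC that ping-pongs back and forth along the spline of a referenced BPSpline actor.
; Each Tick it snaps to the world-space location at its current spline distance, then advances or reduces that distance by speed times delta time.
; The SplineEnd flag flips at either end, with true meaning forward travel.
; Forward travel uses the full spline rotation, while the return leg sets only yaw, turned 180 degrees.
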(event `TurtleMove`
  (`self.Update Position`)
  (if (`self.SplineEnd`)
    ;[1 0.2356 0.1858] Count Distance High
    (if (< (`self.SplineDistanceAlong`) (`SplineComponent.GetSplineLength` (`/Game/01_DEV/NPC/BP_Spline.Spline` (`self.BP_Spline`))))
      (set `self.SplineDistanceAlong` (+ (`self.SplineDistanceAlong`) (* (`GameplayStatics.GetWorldDeltaSeconds`) (`self.SplineSpeed`))))
      (else
        (set `self.SplineEnd` false)))
    (else
      ;[1 0.2081 0.228] Count Distance Down
      (if (> (`self.SplineDistanceAlong`) 0.0)
        (set `self.SplineDistanceAlong` (- (`self.SplineDistanceAlong`) (* (`GameplayStatics.GetWorldDeltaSeconds`) (`self.SplineSpeed`))))
        (else
          (set `self.SplineEnd` true))))))

(event `self.ReceiveTick`
  (params (DeltaSeconds :type "Float (single-precision)"))
  (`self.TurtleMove`))

(event `Update Position`
  (bind _splinedistancealong (`self.SplineDistanceAlong`))
  (bind _spline (`/Game/01_DEV/NPC/BP_Spline.Spline` (`self.BP_Spline`)))
  (bind _returnvalue (`SplineComponent.GetRotationAtDistanceAlongSpline` _spline _splinedistancealong "World"))
  ;[1 1 1] CustomEvent = Holen uns die Spile/Schiene, ruft die Position/Rotation selbst ab
  (`self.K2_SetActorLocation` (`SplineComponent.GetLocationAtDistanceAlongSpline` _spline _splinedistancealong "World"))
  (if (`self.SplineEnd`)
    (bind _output_get (set `self.SplineRotation` _returnvalue))
    (`self.K2_SetActorRotation` _output_get)
    (else
      (bind _output_get_2 (set `self.SplineRotation` _returnvalue))
      (`self.K2_SetActorRotation` (`KismetMathLibrary.MakeRotator` 0.0 0.0 (+ (.yaw _output_get_2) 180.0))))))

(fn `UserConstructionScript`)