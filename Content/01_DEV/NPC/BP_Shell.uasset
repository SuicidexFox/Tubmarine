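; BP_Shell is an NPC hazard that periodically activates and launches BP_Nils along its own forward vector when it overlaps the shell's HitBox.
; After a random delay of a few seconds, a timeline raises the mesh's emissive as a warning.
; It then fades the glow while playing a montage, Niagara effect and sound with an enlarged hit sphere.
; Montage completion shrinks the sphere and restarts the cycle.
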(event `self.ReceiveBeginPlay`
  (`self.SetupRandomAction`))

(event `self.HitBox.OnComponentBeginOverlap`
  (params (OverlappedComponent :type "PrimitiveComponent Object Reference") (OtherActor :type "Actor Object Reference") (OtherComp :type "PrimitiveComponent Object Reference") (OtherBodyIndex :type Integer) (bFromSweep :type Boolean) (SweepResult :type "HitResult Structure (by ref)"))
  ;[1 0.8137 0.1823] Bounce
  (bind _asbp_nils (cast `/Game/01_DEV/Nils/BP_Nils` OtherActor))
  (`Character.LaunchCharacter` _asbp_nils (* (`self.GetActorForwardVector` _asbp_nils) (`self.Bounce`)) true true))

(event `SetupRandomAction`
  ;[1 1 1] RandomAction
  (`KismetSystemLibrary.Delay` (`KismetMathLibrary.Conv_IntToDouble` (`KismetMathLibrary.RandomIntegerInRange` 2 7)))
  (`self.Action`))

(event `Action`
  (bind _schell (`self.Schell`))
  ;[1 1 1] Material
  (bind (_direction _color) (`Timeline|RedFlagTime` :!via `PlayFromStart`)
    (:`Update`
      (`MeshComponent.SetScalarParameterValueOnMaterials` _schell "Emissive" (`KismetMathLibrary.Lerp` 0.0 0.5 _color)))
    (:`Finished`
      (`|ExecutionSequence`
        (:`then_0`
          (bind (_direction_2 _color_2) (`Timeline|RedFlagBackTime` :!via `PlayFromStart`)
            (:`Update`
              (`MeshComponent.SetScalarParameterValueOnMaterials` _schell "Emissive" (`KismetMathLibrary.Lerp` 0.5 0.0 _color_2)))))
        (:`then_1`
          (`|PlayMontage` (`self.Schell`) "/Game/03_3D/NPC/Shell/AM_Action.AM_Action"
            (:`OnCompleted`
              (`SphereComponent.SetSphereRadius` (`self.HitBox`) (`KismetMathLibrary.Lerp` 60.0 1.0 1.5) true)
              (`self.SetupRandomAction`))))
        (:`then_2`
          (`SphereComponent.SetSphereRadius` (`self.HitBox`) (`KismetMathLibrary.Lerp` 1.0 60.0 1.5) true)
          (`NiagaraComponent.ResetSystem` (`self.NS_Shell`))
          (`FMODAudioComponent.Play` (`self.AudioMainMenu`)))))))

(fn `UserConstructionScript`)