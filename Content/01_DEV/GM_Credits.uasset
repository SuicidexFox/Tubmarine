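; Credits game mode that runs the timed credits scene, with fade helpers and a return to the main menu.
; BeginPlay starts the fade and staggers four BP_ActorCreditsSorter entries ten seconds apart, each scaling its bubbles fifteen seconds after activation.
; After fifteen seconds it shows WBP_Credits with UI-only input and activates BP_Title.
; FadeIn uses WBPBasic before SetupWidget creates it; FadeOut opens L_MainMenu but is not called here.
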(event `self.ReceiveBeginPlay`
  (`self.FadeIn`)
  (`self.Actor of Credits`)
  (`KismetSystemLibrary.Delay` 15.0)
  (`self.SetupWidget`)
  (bind _returnvalue (`GameplayStatics.GetActorOfClass` "/Game/05_UI/BP_Title.BP_Title_C"))
  (set `/Game/05_UI/BP_Title.Activate` true _returnvalue))

(event `Actor of Credits`
  (bind _returnvalue (`GameplayStatics.GetActorOfClass` "/Game/05_UI/BP_ActorCreditsSorter.BP_ActorCreditsSorter_C"))
  (`|ExecutionSequence`
    (:`then_0`
      (bind _sorter (`/Game/05_UI/BP_ActorCreditsSorter.Sorter` _returnvalue))
      (bind _output (`|GetArrayItem` _sorter))
      (set `/Game/05_UI/BP_ActorCredits.Activate` true _output)
      (`KismetSystemLibrary.Delay` 15.0)
      (`/Game/05_UI/BP_ActorCredits.BubbsleScale` _output))
    (:`then_1`
      (`KismetSystemLibrary.Delay` 10.0)
      (bind _output_2 (`|GetArrayItem` _sorter 1))
      (set `/Game/05_UI/BP_ActorCredits.Activate` true _output_2)
      (`KismetSystemLibrary.Delay` 15.0)
      (`/Game/05_UI/BP_ActorCredits.BubbsleScale` _output_2))
    (:`then_2`
      (`KismetSystemLibrary.Delay` 20.0)
      (bind _output_3 (`|GetArrayItem` _sorter 2))
      (set `/Game/05_UI/BP_ActorCredits.Activate` true _output_3)
      (`KismetSystemLibrary.Delay` 15.0)
      (`/Game/05_UI/BP_ActorCredits.BubbsleScale` _output_3))
    (:`then_3`
      (`KismetSystemLibrary.Delay` 30.0)
      (bind _output_4 (`|GetArrayItem` _sorter 3))
      (set `/Game/05_UI/BP_ActorCredits.Activate` true _output_4)
      (`KismetSystemLibrary.Delay` 15.0)
      (`/Game/05_UI/BP_ActorCredits.BubbsleScale` _output_4))))

(event `SetupWidget`
  (bind _returnvalue (`GameplayStatics.GetPlayerController` 0))
  ;[1 0.9278 0.349] Credits
  (bind _returnvalue_2 (`|CreateWidget` "/Game/05_UI/WBP_Basic.WBP_Basic_C"))
  (bind _output_get (set `self.WBP_Basic` _returnvalue_2))
  (`UserWidget.AddToPlayerScreen` _output_get 0)
  (`CommonActivatableWidgetContainerBase.BP_AddWidget` (`/Game/05_UI/WBP_Basic.Info_Stack` _output_get) "/Game/05_UI/WBP_Credits.WBP_Credits_C")
  (`WidgetBlueprintLibrary.SetInputMode_UIOnlyEx` _returnvalue null)
  (set `PlayerController.bShowMouseCursor` true _returnvalue))

(event `FadeIn`
  (bind _info_stack (`/Game/05_UI/WBP_Basic.Info_Stack` (`self.WBP_Basic`)))
  ;[0.4072 0.04667 0] Fade
  (bind _returnvalue (`CommonActivatableWidgetContainerBase.BP_AddWidget` _info_stack "/Game/05_UI/WBP_Fade.WBP_Fade_C"))
  (bind _fadein (`/Game/05_UI/WBP_Fade.FadeIn` _returnvalue))
  (`UserWidget.PlayAnimationForward` _returnvalue _fadein 1.0 false)
  (`KismetSystemLibrary.Delay` (`WidgetAnimation.GetEndTime` _fadein))
  (`CommonActivatableWidgetContainerBase.ClearWidgets` _info_stack))

(event `FadeOut`
  (bind _info_stack (`/Game/05_UI/WBP_Basic.Info_Stack` (`self.WBP_Basic`)))
  ;[0.4072 0.04667 0] Fade
  (bind _returnvalue (`CommonActivatableWidgetContainerBase.BP_AddWidget` _info_stack "/Game/05_UI/WBP_Fade.WBP_Fade_C"))
  (bind _fadeout (`/Game/05_UI/WBP_Fade.FadeOut` _returnvalue))
  (`UserWidget.PlayAnimationForward` _returnvalue _fadeout 1.0 false)
  (`KismetSystemLibrary.Delay` (`WidgetAnimation.GetEndTime` _fadeout))
  (`CommonActivatableWidgetContainerBase.ClearWidgets` _info_stack)
  (`GameplayStatics.OpenLevelBySoftObjectPtr` "/Game/08_Scenes/L_MainMenu.L_MainMenu"))

(fn `UserConstructionScript`)