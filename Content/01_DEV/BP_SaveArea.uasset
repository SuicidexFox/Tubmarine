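; BP_SaveArea is an actor that, by its name, marks a save area, with a sphere whose radius is set from SphereRadius on BeginPlay.
; Its Interact function returns false for Friend, H2O and Collactable, and its SaveArea function has no logic.
; Leftover, unreachable nodes would build a SpawnTransform from a save area's location and yaw at unit scale, so no saving happens here.
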(event `self.ReceiveBeginPlay`
  (`SphereComponent.SetSphereRadius` (`self.Sphere`) (`self.SphereRadius`) true))

(fn `Interact`
  (returns (Friend :type Boolean) (H2O :type Boolean) (Collactable :type Boolean))
  (return false false false))

(fn `SaveArea`
  (returns (Actor :type "Actor Object Reference"))
  (return null))

(fn `UserConstructionScript`)