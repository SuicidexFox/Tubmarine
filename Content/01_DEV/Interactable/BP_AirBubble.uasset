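; Collectible air bubble that BP_Nils picks up to raise the HUD air counter.
; While idle, a looping timeline bobs the sphere, choosing a new random height each cycle.
; On capsule overlap, unless the HUD counter equals seven, it calls AirUp on the HUD, plays a 2D sound event and removes the billboard and capsule.
; A collect timeline then shrinks the actor before destroying it.
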(event `self.ReceiveBeginPlay`
  (`self.IdleAnimation`)
  (set `self.OriginPoint` (`self.K2_GetActorLocation`)))

(event `IdleAnimation`
  ;[0.1101 0.4896 0.1497] Animation
  (bind _output_get (set `self.B` (`KismetMathLibrary.MakeVector` 0.0 0.0 (`KismetMathLibrary.Conv_IntToDouble` (`KismetMathLibrary.RandomIntegerInRange` 10 30)))))
  (bind (_direction _idle_bounce) (`Timeline|Idle Animation` :!via `PlayFromStart`)
    (:`Update`
      (`SceneComponent.K2_SetRelativeLocation` (`self.Sphere`) (`KismetMathLibrary.VLerp` (0.0 0.0 0.0) _output_get _idle_bounce) false false))
    (:`Finished`
      (`self.IdleAnimation`))))

(event `self.Capsule.OnComponentBeginOverlap`
  (params (OverlappedComponent :type "PrimitiveComponent Object Reference") (OtherActor :type "Actor Object Reference") (OtherComp :type "PrimitiveComponent Object Reference") (OtherBodyIndex :type Integer) (bFromSweep :type Boolean) (SweepResult :type "HitResult Structure (by ref)"))
  ;[1 0.3698 0.3904] Wenn Player den Collider trifft
  (bind _asbp_nils (cast `/Game/01_DEV/Nils/BP_Nils` OtherActor))
  (bind _wbp_hud (`/Game/01_DEV/GM_Tub.WBP_HUD` (`/Game/01_DEV/Nils/BP_Nils.GM Tub` _asbp_nils)))
  (if (not (== (`/Game/05_UI/WBP_HUD.CounterAirBubble` _wbp_hud) 7))
    (`self.DestroyAir` _wbp_hud)
    (`FMODBlueprintStatics.PlayEvent2D` "/Game/FMOD/Events/SFX/UI/TakeBubble.TakeBubble")
    (`ActorComponent.K2_DestroyComponent` (`self.Billboard`))
    (`ActorComponent.K2_DestroyComponent` (`self.Capsule`))))

(event `DestroyAir`
  (params (Actor :type "/Game/05_UI/WBP_HUD Object Reference"))
  ;[1 0.3698 0.3904] Wenn Player den Collider trifft
  (`/Game/05_UI/WBP_HUD.AirUp` Actor)
  (bind (_direction _shrink) (`Timeline|CollectAnimation`)
    (:`Update`
      (`self.K2_SetActorLocation` (`KismetMathLibrary.VLerp` (`self.OriginPoint`) (`self.K2_GetActorLocation`) _shrink)) ; Ort
      (`self.SetActorScale3D` (`KismetMathLibrary.VLerp` (1.0 1.0 1.0) (0.0 0.0 0.0) _shrink)) ; Größe
    )
    (:`Finished`
      (`self.K2_DestroyActor`))))

(fn `UserConstructionScript`)