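; BP_Tilli is an interactable actor that plays a cutscene when BP_Nils overlaps it.
; It calls TutorialSupport on Nils's GMTub, then after a brief delay zeroes PercentTime, toggles input off and starts its level sequence.
; Meanwhile it calls Mesh1 on Nils and removes its Animal component.
; When the sequence's duration has passed, it re-enables input, sets PercentTime to a small nonzero value and destroys itself.
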(event `self.ReceiveActorBeginOverlap`
  (params (OtherActor :type "Actor Object Reference"))
  (bind _returnvalue (`GameplayStatics.GetPlayerController` 0))
  (bind _sequenceplayer (`LevelSequenceActor.SequencePlayer` (`self.LevelSequence`)))
  (bind _asbp_nils (cast `/Game/01_DEV/Nils/BP_Nils` OtherActor))
  (`/Game/01_DEV/GM_Tub.TutorialSupport` (`/Game/01_DEV/Nils/BP_Nils.GM Tub` _asbp_nils))
  (`KismetSystemLibrary.Delay` 0.1)
  (`|ExecutionSequence`
    (:`then_0`
      (bind _gm_tub (`/Game/01_DEV/Nils/BP_Nils.GM Tub` _asbp_nils))
      (set `/Game/01_DEV/GM_Tub.PercentTime` 0.0 _gm_tub)
      (`self.DisableInput` _returnvalue)
      (`MovieSceneSequencePlayer.Play` _sequenceplayer)
      (`KismetSystemLibrary.Delay` (`TimeManagementBlueprintLibrary.Conv_QualifiedFrameTimeToSeconds` (`MovieSceneSequencePlayer.GetEndTime` _sequenceplayer)))
      (`self.EnableInput` _returnvalue null)
      (set `/Game/01_DEV/GM_Tub.PercentTime` 0.01 _gm_tub)
      (`self.K2_DestroyActor`))
    (:`then_1`
      (`/Game/01_DEV/Nils/BP_Nils.Mesh_1` _asbp_nils)
      (`ActorComponent.K2_DestroyComponent` (`self.Animal`)))))

(fn `Input`
  (returns (Jump :type Boolean) (Up :type Boolean))
  (return false false))

(fn `Interact`
  (returns (Collect :type Boolean) (CollectID :type "StaticMesh Object Reference"))
  (return false null))

(fn `StartLevelSequence`
  (returns (Delay :type "Float (double-precision)"))
  (return 0.0))

(fn `UserConstructionScript`)