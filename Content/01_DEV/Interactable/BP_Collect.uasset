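; BP_Collect is an interactable duck collectible that shows a button prompt when approached and hides it on leave.
; Its Interact function reports the collect flag and the duck's static mesh, cached at BeginPlay as the ID.
; Help plays the Ducks 2D sound event and destroys the actor.
; An AnyKey handler swaps the prompt sprite to match keyboard or gamepad input, while Input and StartLevelSequence return only default values.
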(event `self.ReceiveBeginPlay`
  (set `self.DuckID` (`StaticMeshComponent.StaticMesh` (`self.Duck`))))

(event `/Game/01_DEV/Interface/BPI_Interactables.Approache`
  (`SceneComponent.SetHiddenInGame` (`self.Billboard`) false false))

(event `/Game/01_DEV/Interface/BPI_Interactables.Leave`
  (`SceneComponent.SetHiddenInGame` (`self.Billboard`) true false))

(event `/Game/01_DEV/Interface/BPI_Interactables.Help`
  (`FMODBlueprintStatics.PlayEvent2D` "/Game/FMOD/Events/SFX/UI/Ducks.Ducks")
  (`self.K2_DestroyActor`))

(event `Key|AnyKey`
  (params (Key :type "Key Structure"))
  (bind _billboard (`self.Billboard`))
  ;[0.1458 0.1458 0.1458] Input
  (:`Pressed`
    (if (`KismetInputLibrary.Key_IsKeyboardKey` Key)
      (`BillboardComponent.SetSprite` _billboard "/Game/05_UI/Buttons/Icons/Billboard_Keyboard.Billboard_Keyboard")
      (elif (`KismetInputLibrary.Key_IsGamepadKey` Key)
        (`BillboardComponent.SetSprite` _billboard "/Game/05_UI/Buttons/Icons/Billboard_Controller.Billboard_Controller")))))

(fn `Input`
  (returns (Jump :type Boolean) (Up :type Boolean))
  (return false false))

(fn `Interact`
  (returns (Collect :type Boolean) (CollectID :type "StaticMesh Object Reference"))
  (return (`self.IsCollect`) (`self.DuckID`)))

(fn `StartLevelSequence`
  (returns (Delay :type "Float (double-precision)"))
  (return 0.0))

(fn `UserConstructionScript`)