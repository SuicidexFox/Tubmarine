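; Spawner actor that keeps a BP_AirBubble at its location, creating the first on BeginPlay and storing it as the current bubble.
; Tick polls that reference, and when it is empty a DoOnce gate starts a SpawnRate delay before spawning a replacement at the saved transform.
; A second Tick check is meant to reset the gate once a bubble is present again.
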(event `self.ReceiveBeginPlay`
  (bind _output_get (set `self.SpawnerTransform` (`self.GetTransform`)))
  (bind _returnvalue (`|SpawnActorFromClass` "/Game/01_DEV/Interactable/BP_AirBubble.BP_AirBubble_C" _output_get "Undefined" "MultiplyWithRoot" null null))
  (set `self.CurrentAirBubble` _returnvalue))

(event `self.ReceiveTick`
  (params (DeltaSeconds :type "Float (single-precision)"))
  (`|ExecutionSequence`
    (:`then_0`
      (if (== (`self.CurrentAirBubble`) null)
        (`/Engine/EditorBlueprintResources/StandardMacros.DoOnce` false :!label _label
          (:`Completed`
            (`KismetSystemLibrary.Delay` (`self.SpawnRate`))
            (bind _returnvalue (`|SpawnActorFromClass` "/Game/01_DEV/Interactable/BP_AirBubble.BP_AirBubble_C" (`self.SpawnerTransform`) "Undefined" "MultiplyWithRoot" null null))
            (set `self.CurrentAirBubble` _returnvalue)))))
    (:`then_1`
      (if (== (`self.CurrentAirBubble`) "/Game/01_DEV/Interactable/BP_AirBubble.BP_AirBubble")
        (goto _label :!via `Reset`)))))

(fn `UserConstructionScript`)