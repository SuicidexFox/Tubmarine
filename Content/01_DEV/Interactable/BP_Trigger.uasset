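; BP_Trigger is an interactable that shows a billboard prompt on approach, hides it on leave, and removes it when help is given.
; Any mouse button or gamepad press switches the prompt sprite between keyboard and controller versions.
; It reports its jump, up and collect flags, and can restore a linked stone's material.
; StartLevelSequence plays its sequence, returns the length, and destroys the actor after that delay.
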(event `/Game/01_DEV/Interface/BPI_Interactables.Help`
  ;[1 1 1] Instance
  (set `self.Trigger_AnimationSupport` true)
  (`ActorComponent.K2_DestroyComponent` (`self.Billboard`)))

(event `self.Approache`
  ;[1 1 1] Instance
  (`SceneComponent.SetHiddenInGame` (`self.Billboard`) false false))

(event `self.Leave`
  ;[1 1 1] Instance
  (`SceneComponent.SetHiddenInGame` (`self.Billboard`) true false))

(event `SetMaterial`
  (`PrimitiveComponent.SetMaterial` (`/Game/01_DEV/Interactable/BP_Rock.Stone` (`self.Stone`)) 0 "/Game/04_Material/World/M_Stones.M_Stones"))

(event `Destroy`
  (`KismetSystemLibrary.Delay` (`self.Delay`))
  (`self.K2_DestroyActor`))

(event `Key|AnyKey`
  (params (Key :type "Key Structure"))
  (bind _billboard (`self.Billboard`))
  ;[0.1458 0.1458 0.1458] Input
  (:`Pressed`
    (if (`KismetInputLibrary.Key_IsMouseButton` Key)
      (`BillboardComponent.SetSprite` _billboard "/Game/05_UI/Buttons/Icons/Billboard_Keyboard.Billboard_Keyboard")
      (elif (`KismetInputLibrary.Key_IsGamepadKey` Key)
        (`BillboardComponent.SetSprite` _billboard "/Game/05_UI/Buttons/Icons/Billboard_Controller.Billboard_Controller")))))

(fn `Input`
  (returns (Jump :type Boolean) (Up :type Boolean))
  (return (`self.ActivateJump`) (`self.ActivateUp`)))

(fn `Interact`
  (returns (Collect :type Boolean) (CollectID :type "StaticMesh Object Reference"))
  (return (`self.IsCollect`) null))

(fn `StartLevelSequence`
  (returns (Delay :type "Float (double-precision)"))
  (bind _sequenceplayer (`LevelSequenceActor.SequencePlayer` (`self.LevelSequence`)))
  (`MovieSceneSequencePlayer.Play` _sequenceplayer)
  (bind _output_get (set `self.Delay` (`TimeManagementBlueprintLibrary.Conv_QualifiedFrameTimeToSeconds` (`MovieSceneSequencePlayer.GetEndTime` _sequenceplayer))))
  (`self.Destroy`)
  (return _output_get))

(fn `UserConstructionScript`)