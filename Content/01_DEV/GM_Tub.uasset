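; Game mode for the Tub level that registers with GI_Base, sets up the duck cam and runs UI, fades, pause and tutorials.
; Widgets go onto stacks in WBP_Basic, while GI_Base flags gate one-time tutorials; only Movement and Respawn are wired, the others are stubbed.
; The respawn flag starts a self-recalling one-second Delay loop draining the HUD percentage.
; GetNextCheckpoint cycles through BP_SpawnPosition transforms, wrapping at the end.
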(event `self.ReceiveBeginPlay`
  (`self.SetupGameInstance`)
  (`self.SetupWidget`)
  (`self.SetupGamemode`)
  (`self.SetupDuckCam`)
  (`self.Checkpoints`)
  (`self.FadeIn`)
  (`FMODAudioComponent.Play` (`self.Atmo`))
  ;[1 1 1] gespeicherte Variable / Timer
  (if (`/Game/01_DEV/GI_Base.T_PlayerRespwan` (`self.GI Base`))
    (`self.Timer`)
    (set `self.Percent` 1.0)))

(event `self.ReceiveEndPlay`
  (params (EndPlayReason :type "EEndPlayReason Enum" :default "Destroyed"))
  (`FMODAudioComponent.Stop` (`self.Atmo`)))

(event `SetupGameInstance`
  ;[1 1 1] GameInstance
  (bind _asgi_base (cast `/Game/01_DEV/GI_Base` (`GameplayStatics.GetGameInstance`)))
  (set `self.GI Base` _asgi_base))

(event `SetupGameMode`
  ;[1 1 1] GameMode
  (`/Game/01_DEV/GI_Base.SetGameMode` (`self.GI Base`) "GM_Tub_C"))

(event `SetupWidget`
  ;[1 1 1] Widget
  (bind _returnvalue (`|CreateWidget` "/Game/05_UI/WBP_Basic.WBP_Basic_C"))
  (bind _output_get (set `self.WBP Basic` _returnvalue))
  (`UserWidget.AddToPlayerScreen` _output_get 0))

(event `SetupDuckCam`
  ;[1 1 1] DuckCam
  (bind _returnvalue (`GameplayStatics.GetActorOfClass` "/Game/05_UI/Ducks/BP_UI_Duck.BP_UI_Duck_C"))
  (`/Game/01_DEV/GI_Base.SetupDuckCam` (`self.GI Base`) _returnvalue))

(event `Checkpoints`
  ;[1 1 1] Checkpoints
  (bind _outactors (`GameplayStatics.GetAllActorsOfClass` "/Game/01_DEV/Nils/BP_SpawnPosition.BP_SpawnPosition_C"))
  (set `self.CheckpointList` _outactors))

(event `AudioUI`
  ;[1 1 1] Audio
  (`FMODBlueprintStatics.PlayEvent2D` "/Game/FMOD/Events/SFX/UI/StartGame.StartGame"))

(event `TogglePause`
  (bind _returnvalue (`GameplayStatics.GetPlayerController` 0))
  ;[1 1 1] Toogle
  (`GameplayStatics.SetGamePaused` true)
  (`WidgetBlueprintLibrary.SetInputMode_UIOnlyEx` _returnvalue null)
  (set `PlayerController.bShowMouseCursor` true _returnvalue))

(event `ToggleActive`
  ;[1 1 1] PlayerInput
  (`self.EnableInput` (`GameplayStatics.GetPlayerController` 0) null))

(event `ToggleDeactive`
  ;[1 1 1] PlayerInput
  (`self.DisableInput` (`GameplayStatics.GetPlayerController` 0) null))

(event `ToggleGame`
  (bind _returnvalue (`GameplayStatics.GetPlayerController` 0))
  ;[1 1 1] Toogle
  (`GameplayStatics.SetGamePaused` false)
  (`WidgetBlueprintLibrary.SetInputMode_GameOnly` _returnvalue)
  (set `PlayerController.bShowMouseCursor` false _returnvalue))

(event `SetupHUD`
  ;[1 0.1152 0] HUD
  (bind _returnvalue (`CommonActivatableWidgetContainerBase.BP_AddWidget` (`/Game/05_UI/WBP_Basic.HUD_Stack` (`self.WBP Basic`)) "/Game/05_UI/WBP_HUD.WBP_HUD_C"))
  (set `self.WBP_HUD` _returnvalue))

(event `Fade`
  (bind _info_stack (`/Game/05_UI/WBP_Basic.Info_Stack` (`self.WBP Basic`)))
  ;[0.4072 0.04667 0] Fade
  (`self.ToggleDeactive`)
  (bind _returnvalue (`CommonActivatableWidgetContainerBase.BP_AddWidget` _info_stack "/Game/05_UI/WBP_Fade.WBP_Fade_C"))
  (bind _fade (`/Game/05_UI/WBP_Fade.Fade` _returnvalue))
  (`UserWidget.PlayAnimationForward` _returnvalue _fade 1.0 false)
  (`KismetSystemLibrary.Delay` (`WidgetAnimation.GetEndTime` _fade))
  (`CommonActivatableWidgetContainerBase.ClearWidgets` _info_stack))

(event `SaveAreaUI`
  ;[1 0.1152 0] HUD
  (`/Game/05_UI/WBP_HUD.VisibleSaveArea` (`self.WBP_HUD`)))

(event `FadeIn`
  (bind _info_stack (`/Game/05_UI/WBP_Basic.Info_Stack` (`self.WBP Basic`)))
  ;[0.4072 0.04667 0] Fade
  (`self.ToggleDeactive`)
  (bind _returnvalue (`CommonActivatableWidgetContainerBase.BP_AddWidget` _info_stack "/Game/05_UI/WBP_Fade.WBP_Fade_C"))
  (bind _fadein (`/Game/05_UI/WBP_Fade.FadeIn` _returnvalue))
  (`UserWidget.PlayAnimationForward` _returnvalue _fadein 1.0 false)
  (`KismetSystemLibrary.Delay` (`WidgetAnimation.GetEndTime` _fadein))
  (`CommonActivatableWidgetContainerBase.ClearWidgets` _info_stack)
  (`self.ToggleActive`)
  (`self.ToggleGame`)
  (if (`/Game/01_DEV/GI_Base.T_Move` (`self.GI Base`))
    (`self.SetupHUD`)
    (else
      (`self.TutorialMove`))))

(event `CollectUI`
  ;[1 0.1152 0] HUD
  (`/Game/05_UI/WBP_HUD.VisibleCollect` (`self.WBP_HUD`)))

(event `Timer`
  ;[1 0.1152 0] HUD
  ;;[1 1 1] Timeline
  (bind _output_get (set `self.Percent` (- (`self.Percent`) (`self.PercentTime`))))
  (`/Game/05_UI/WBP_HUD.SetPercent` (`self.WBP_HUD`) _output_get)
  (`KismetSystemLibrary.Delay` 1.0)
  (`self.Timer`))

(event `FadeOut`
  ;[0.4072 0.04667 0] Fade
  (bind _returnvalue (`CommonActivatableWidgetContainerBase.BP_AddWidget` (`/Game/05_UI/WBP_Basic.Info_Stack` (`self.WBP Basic`)) "/Game/05_UI/WBP_Fade.WBP_Fade_C"))
  (`UserWidget.PlayAnimationForward` _returnvalue (`/Game/05_UI/WBP_Fade.FadeOut` _returnvalue) 1.0 false)
  (`KismetSystemLibrary.Delay` 2.0)
  (`GameplayStatics.OpenLevelBySoftObjectPtr` "/Game/08_Scenes/L_MainMenu.L_MainMenu"))

(event `SetupPause`
  ;[1 1 1] Pause
  (`self.AudioUI`)
  (bind _returnvalue (`CommonActivatableWidgetContainerBase.BP_AddWidget` (`/Game/05_UI/WBP_Basic.Menu_Stack` (`self.WBP Basic`)) "/Game/05_UI/WBP_Pause_Basic.WBP_Pause_Basic_C"))
  (`CommonActivatableWidgetContainerBase.BP_AddWidget` (`/Game/05_UI/WBP_Pause_Basic.Pause_Stack` _returnvalue) "/Game/05_UI/WBP_Pause.WBP_Pause_C")
  (`self.TogglePause`)
  (`FMODAudioComponent.Stop` (`self.HUDSound`)))

(event `Continue`
  ;[1 1 1] Pause
  (`self.AudioUI`)
  (`CommonActivatableWidgetContainerBase.ClearWidgets` (`/Game/05_UI/WBP_Basic.Menu_Stack` (`self.WBP Basic`)))
  (`self.ToggleGame`)
  (`/Game/05_UI/WBP_HUD.ResetDoOnce` (`self.WBP_HUD`)))

(event `TutorialMove`
  (bind _gi_base (`self.GI Base`))
  (if (not (`/Game/01_DEV/GI_Base.T_Move` _gi_base))
    (set `/Game/01_DEV/GI_Base.T_Move` true _gi_base)
    (`CommonActivatableWidgetContainerBase.BP_AddWidget` (`/Game/05_UI/WBP_Basic.Info_Stack` (`self.WBP Basic`)) "/Game/05_UI/Tutorial/WBP_Tutorial_01_Movement.WBP_Tutorial_01_Movement_C")
    (`self.TogglePause`)
    (`self.AudioUI`)))

(event `TutorialJump`)

(event `TutorialSave`
  (bind _gi_base (`self.GI Base`))
  (if (not (`/Game/01_DEV/GI_Base.T_PlayerRespwan` _gi_base))
    (set `/Game/01_DEV/GI_Base.T_PlayerRespwan` true _gi_base)
    (`self.Timer`)
    (`CommonActivatableWidgetContainerBase.BP_AddWidget` (`/Game/05_UI/WBP_Basic.Info_Stack` (`self.WBP Basic`)) "/Game/05_UI/Tutorial/WBP_Tutorial_03_Respawn.WBP_Tutorial_03_Respawn_C")
    (`self.TogglePause`)
    (`self.AudioUI`)))

(event `TutorialSupport`)

(event `TutorialUp`)

(event `TutorialDucks`)

(fn `GetNextCheckpoint`
  (returns (`Teleport Point` :type "Transform Structure"))
  (locals (CheckpointStart :type "Transform Structure"))
  (bind _chekpointid (`self.ChekpointID`))
  (set `local.CheckpointStart` (`SceneComponent.K2_GetComponentToWorld` (`/Game/01_DEV/Nils/BP_SpawnPosition.Arrow` (`|GetArrayItem` (`self.CheckpointList`) _chekpointid))))
  (bind _result (`/Engine/EditorBlueprintResources/StandardMacros.IncrementInt` _chekpointid)
    (:`  `
      (if (== _result (`KismetArrayLibrary.Array_Length` (`self.CheckpointList`)))
        (set `self.ChekpointID` 0))
      (return (`local.CheckpointStart`)))))

(fn `UserConstructionScript`)