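; BP_AirBubble is a collectible air bubble that bobs in place until it is taken.
; A looping idle timeline moves the BubbleLightBlue component vertically, picking a new random height each time it restarts.
; The Take event plays a collect timeline that pulls the actor from its spawn point toward the given actor while shrinking it to zero, then destroys it.
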(event `self.ReceiveBeginPlay`
  (`self.IdleAnimation`)
  (set `self.OriginPoint` (`self.K2_GetActorLocation`)))

(event `IdleAnimation`
  ;[0.1101 0.4896 0.1497] Animation
  (bind _output_get (set `self.B` (`KismetMathLibrary.MakeVector` 0.0 0.0 (`KismetMathLibrary.Conv_IntToDouble` (`KismetMathLibrary.RandomIntegerInRange` 10 30)))))
  (bind (_direction _idle_bounce) (`Timeline|Idle Animation` :!via `PlayFromStart`)
    (:`Update`
      (`SceneComponent.K2_SetRelativeLocation` (`self.Bubble_LightBlue`) (`KismetMathLibrary.VLerp` (0.0 0.0 0.0) _output_get _idle_bounce) false false))
    (:`Finished`
      (`self.IdleAnimation`))))

(event `/Game/01_DEV/Interface/BPI_AirBubble.Take`
  (params (ID_Actor :type "Actor Object Reference"))
  ;[1 0.3698 0.3904] Wenn Player den Collider trifft
  (bind (_direction _shrink) (`Timeline|CollectAnimation`)
    (:`Update`
      (`self.K2_SetActorLocation` (`KismetMathLibrary.VLerp` (`self.OriginPoint`) (`self.K2_GetActorLocation` ID_Actor) _shrink)) ; Ort
      (`self.SetActorScale3D` (`KismetMathLibrary.VLerp` (1.0 1.0 1.0) (0.0 0.0 0.0) _shrink)) ; Größe
    )
    (:`Finished`
      (`self.K2_DestroyActor`))))

(fn `UserConstructionScript`)