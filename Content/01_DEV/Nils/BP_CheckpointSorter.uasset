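; BP_CheckpointSorter holds the checkpoint list for the level and hands it to the game mode.
; On BeginPlay it casts the game mode to GM_Tub and copies its CeckpointID array into CheckpointList.
; It then counts the BP_SpawnPosition actors in the level and prints a debug message when that count differs from the list length.
; The script does no sorting itself, so the array is passed on as stored.
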(event `self.ReceiveBeginPlay`
  (bind _returnvalue (`KismetArrayLibrary.Array_Length` (`self.CeckpointID`)))
  (bind _asgm_tub (cast `/Game/01_DEV/GM_Tub` (`GameplayStatics.GetGameMode`)))
  (set `/Game/01_DEV/GM_Tub.CheckpointList` (`self.CeckpointID`) _asgm_tub)
  (bind _outactors (`GameplayStatics.GetAllActorsOfClass` "/Game/01_DEV/Nils/BP_SpawnPosition.BP_SpawnPosition_C"))
  (bind _returnvalue_2 (`KismetArrayLibrary.Array_Length` _outactors))
  (if (not (== _returnvalue_2 _returnvalue))
    (`KismetSystemLibrary.PrintString` (`KismetTextLibrary.Conv_TextToString` (`|FormatText` "Checkpoint {Actor of Class} out of {List} Checkpoints" _returnvalue_2 _returnvalue)))))

(fn `UserConstructionScript`)