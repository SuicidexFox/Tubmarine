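; BP_Title is a credits title actor that travels along a spline and removes itself at the end.
; While Activate is set, each tick places the actor at the world location for its current Distance on the referenced spline.
; It then advances Distance by Speed times delta seconds, destroying the actor once Distance reaches the spline length.
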(event `self.ReceiveTick`
  (params (DeltaSeconds :type "Float (single-precision)"))
  (if (`self.Activate`)
    (`self.Update Position`)
    (`self.TitleMove`)))

(event `TitleMove`
  (if (>= (`self.Distance`) (`SplineComponent.GetSplineLength` (`/Game/01_DEV/NPC/BP_Spline.Spline` (`self.Spline`))))
    (`self.K2_DestroyActor`)
    (else
      (set `self.Distance` (+ (`self.Distance`) (* (`GameplayStatics.GetWorldDeltaSeconds`) (`self.Speed`)))))))

(event `Update Position`
  ;[1 1 1] Position
  (`self.K2_SetActorLocation` (`SplineComponent.GetLocationAtDistanceAlongSpline` (`/Game/01_DEV/NPC/BP_Spline.Spline` (`self.Spline`)) (`self.Distance`) "World")))

(fn `UserConstructionScript`)