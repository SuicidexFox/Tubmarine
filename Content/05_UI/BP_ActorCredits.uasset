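; BP_ActorCredits is an actor, apparently a bubble for the credits, that travels along a referenced spline.
; While Activate is set, Tick places it at the current Distance along the spline in world space, then advances Distance by Speed times delta time.
; It destroys itself at the spline's end.
; A separate BubbsleScale event, not called here, repeatedly shrinks the BubbleDarkBlue component through a delayed self-call with no stop condition.
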(event `self.ReceiveTick`
  (params (DeltaSeconds :type "Float (single-precision)"))
  (if (`self.Activate`)
    (`self.Update Position`)
    (`self.BubbleMove`)))

(event `BubbleMove`
  (if (>= (`self.Distance`) (`SplineComponent.GetSplineLength` (`/Game/01_DEV/NPC/BP_Spline.Spline` (`self.Spline`))))
    (`self.K2_DestroyActor`)
    (else
      (set `self.Distance` (+ (`self.Distance`) (* (`GameplayStatics.GetWorldDeltaSeconds`) (`self.Speed`)))))))

(event `Update Position`
  ;[1 1 1] Position
  (`self.K2_SetActorLocation` (`SplineComponent.GetLocationAtDistanceAlongSpline` (`/Game/01_DEV/NPC/BP_Spline.Spline` (`self.Spline`)) (`self.Distance`) "World")))

(event `BubbsleScale`
  (bind _bubble_darkblue (`self.Bubble_DarkBlue`))
  (`SceneComponent.SetWorldScale3D` _bubble_darkblue (- (`SceneComponent.RelativeScale3D` _bubble_darkblue) (0.1 0.1 0.1)))
  (`KismetSystemLibrary.Delay` 0.08)
  (`self.BubbsleScale`))

(fn `UserConstructionScript`)