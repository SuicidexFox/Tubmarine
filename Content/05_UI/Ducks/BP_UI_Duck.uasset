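; BP_UI_Duck is a display actor that shows a continuously spinning duck mesh, apparently for the UI.
; From BeginPlay, a self-recalling Rotate event adds a small yaw step to DuckDummy's world rotation after each short Delay rather than using Tick.
; The CurrentStaticMash event swaps the static mesh shown on DuckDummy.
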(event `self.ReceiveBeginPlay`
  (`self.Rotate`))

(event `Rotate`
  (bind _duck_dummy (`self.Duck_Dummy`))
  (bind (_returnvalue_roll _returnvalue_pitch _returnvalue_yaw) (`KismetMathLibrary.BreakRotator` (`SceneComponent.K2_GetComponentRotation` _duck_dummy)))
  (`SceneComponent.K2_SetWorldRotation` _duck_dummy (`KismetMathLibrary.MakeRotator` _returnvalue_roll _returnvalue_pitch (+ _returnvalue_yaw 1.0)) false false)
  (`KismetSystemLibrary.Delay` 0.02)
  (`self.Rotate`))

(event `CurrentStaticMash`
  (params (StaticMash :type "StaticMesh Object Reference"))
  (`StaticMeshComponent.SetStaticMesh` (`self.Duck_Dummy`) StaticMash))

(fn `UserConstructionScript`)